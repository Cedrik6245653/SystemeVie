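; Player state Blueprint that owns the player's health component and persists health through the game instance.
; On BeginPlay it either restores current and max health from the game instance or, on first run, resets health and flags it as initialized.
; Health change events write both values back to the game instance.
; On death it asks the game mode to start respawn for player controller 0.
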(event OnDeath(AC_Health)
  (bind _asbp_new_tpgame_mode (Utilities|Casting|CastToBP_NewTPGameMode (Game|GetGameMode)))
  (Default|StartRespawn _asbp_new_tpgame_mode (Game|GetPlayerController 0)))

(event OnHealthChanged(AC_Health)
  (params (Current%20Health :type Float%20%28double-precision%29) (Max%20Health :type Float%20%28double-precision%29))
  (CallFunction|SaveCurrentHealth Current%20Health)
  (CallFunction|SaveMaxHealth Max%20Health))

(event EventBeginPlay
  (bind _asbp_game_instance (Utilities|Casting|CastToBP_GameInstance (Game|GetGameInstance)))
  (bind _output_get (Variables|Default|SetRefGameInstance _asbp_game_instance))
  (if (Variables|/Game/Game/Blueprints/BP_GameInstance.BP_GameInstance_C|GetHealthInitialized_GI _asbp_game_instance)
    (CallFunction|LoadHealthfromGameInstance)
    (else
      (Class|BPIDamagable|ResetHealth(Message) (Variables|Default|GetAC_Health))
      (Variables|/Game/Game/Blueprints/BP_GameInstance.BP_GameInstance_C|SetHealthInitialized_GI _output_get true))))

(fn ConstructionScript)

(fn SaveCurrentHealth
  (params (New%20Health :type Float%20%28double-precision%29))
  (Variables|/Game/Game/Blueprints/BP_GameInstance.BP_GameInstance_C|SetCurrentHealth_GI (Variables|Default|GetRefGameInstance) New%20Health))

(fn SaveMaxHealth
  (params (New%20Max%20Health :type Float%20%28double-precision%29))
  (Variables|/Game/Game/Blueprints/BP_GameInstance.BP_GameInstance_C|SetMaxHealth_GI (Variables|Default|GetRefGameInstance) New%20Max%20Health))

(fn LoadHealthfromGameInstance
  (bind _refgameinstance (Variables|Default|GetRefGameInstance))
  (bind _ac_health (Variables|Default|GetAC_Health))
  (bind _output_get (Variables|/Game/Game/Blueprints/Components/AC_Health.AC_Health_C|SetMaxHealth _ac_health (Variables|/Game/Game/Blueprints/BP_GameInstance.BP_GameInstance_C|GetMaxHealth_GI _refgameinstance)))
  (bind _output_get_2 (Variables|/Game/Game/Blueprints/Components/AC_Health.AC_Health_C|SetCurrentHealth _ac_health (Variables|/Game/Game/Blueprints/BP_GameInstance.BP_GameInstance_C|GetCurrentHealth_GI _refgameinstance)))
  (Default|CallOnHealthChanged _ac_health _output_get_2 _output_get))