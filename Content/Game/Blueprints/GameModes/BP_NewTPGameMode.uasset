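; Game mode Blueprint that handles player respawning.
; StartRespawn stores the player controller, disables its input, triggers a camera shake and camera fade, then sets a delayed timer.
; The timer calls LoadLevel, which, despite its name, restarts the player without loading a level, re-possesses the controlled pawn, restores input and calls ResetHealthMessage on the PlayerState.
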(event Custom|StartRespawn
  (params (PlayerController :type Player%20Controller%20Object%20Reference))
  (bind _output_get (Variables|Default|SetPlayerController PlayerController))
  (Input|DisableInput _output_get _output_get)
  (Game|Feedback|ClientStartCameraShake _output_get "/Script/Engine.CameraShakeBase" 1.0 "CameraLocal" "0, 0, 0")
  (CameraFades|StartCameraFade :self (Variables|/Script/Engine.PlayerController|GetPlayerCameraManager _output_get) :FromAlpha 1.0 :Duration 1.0 :bHoldWhenFinished true)
  (Utilities|Time|SetTimerbyFunctionName 0 "LoadLevel" 1.5))

(fn ConstructionScript)

(fn LoadLevel
  (bind _playercontroller (Variables|Default|GetPlayerController))
  (Class|GameModeBase|RestartPlayer _playercontroller)
  (Pawn|Possess _playercontroller (Pawn|GetControlledPawn _playercontroller))
  (Input|EnableInput _playercontroller)
  (Class|BPIDamagable|ResetHealth(Message) (Variables|/Script/Engine.Controller|GetPlayerState _playercontroller)))