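; AC_Health is an actor component that tracks health and death state for its owner.
; Damage and healing events are ignored once dead, while a reset clears the dead flag and restores full health.
; All changes pass through one function that clamps health between zero and max, broadcasts a health-changed notification and fires a death notification when health reaches zero.
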(event EventBeginPlay)

(event EventGainHealth
  (params (HealthAmount :type Float%20%28double-precision%29))
  (if (not (Variables|Default|GetIsDead))
    (CallFunction|UpdateHealthandNotify (+ (Variables|Default|GetCurrentHealth) HealthAmount))))

(event EventTakeDamage
  (params (DamageAmount :type Float%20%28double-precision%29))
  (if (not (Variables|Default|GetIsDead))
    (CallFunction|UpdateHealthandNotify (- (Variables|Default|GetCurrentHealth) DamageAmount))))

(event EventResetHealth
  (Variables|Default|SetIsDead false)
  (CallFunction|UpdateHealthandNotify (Variables|Default|GetMaxHealth)))

(fn UpdateHealthandNotify
  (params (NewHealthValue :type Float%20%28double-precision%29))
  (bind _maxhealth (Variables|Default|GetMaxHealth))
  (bind _output_get (Variables|Default|SetCurrentHealth (Math|Float|Clamp(Float) NewHealthValue 0.0 _maxhealth)))
  (Default|CallOnHealthChanged _output_get _maxhealth)
  (bind _output_get_2 (Variables|Default|SetIsDead (<= _output_get 0.0)))
  (if _output_get_2
    (Default|CallOnDeath)))